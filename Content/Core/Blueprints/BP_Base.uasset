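; BP_Base is a team base owned by Hell, Heaven or Neutral players, whose death triggers the victory screen.
; OnDeath chains through S_ and M_ events, apparently server then multicast, to pass PlayerOwner to ServerVictoryScreen on BP_CustomGameState.
; PlayerOwner also selects the static mesh in SetMesh and the cylinder material in the construction script.
; A TestDeath event applies damage for testing.
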(event `self.OnDeath`
  (`self.S_OnDeath`))

(event `S_OnDeath`
  (`self.M_OnDEath`))

(event `M_OnDeath`
  (bind _asbp_custom_game_state (cast `/Game/Core/Blueprints/BP_CustomGameState` (`GameplayStatics.GetGameState`)))
  (`CustomGameState.ServerVictoryScreen` _asbp_custom_game_state (`self.PlayerOwner`)))

(event `self.SetMesh`
  (`StaticMeshComponent.SetStaticMesh` (`self.Mesh`) (select `EPlayer` (`self.PlayerOwner`) :`P_Hell` "/Game/Game_Art/Asset_temp/Porte/SM_Portail_Enfer.SM_Portail_Enfer" :`P_Heaven` "/Game/Game_Art/Assets/pin.pin" :`P_Neutral` "/Game/Game_Art/Asset_temp/Brasero/Brasero_low.Brasero_low" :!type "StaticMesh Object Reference")))

(event `TestDeath`
  (`self.TakeDamage` 100))

(fn `UserConstructionScript`
  (`PrimitiveComponent.SetMaterial` (`self.Cylinder`) 0 (select `EPlayer` (`self.PlayerOwner`) :`P_Hell` "/Game/Core/Texture_DEBUG/Mi_HellPlayer.Mi_HellPlayer" :`P_Heaven` "/Game/Core/Texture_DEBUG/Mi_HeavenPlayer.Mi_HeavenPlayer" :`P_Neutral` "/Game/Core/Texture_DEBUG/M_NeutralPlayer.M_NeutralPlayer" :!type "MaterialInterface Object Reference")))