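; Lobby player pawn with a widget showing the player's Steam name and avatar, plus an authority-only event that server-travels to the minimap level.
; A server event triggers a multicast that loops through the GameState's PlayerArray and fills each lobby pawn's Steam info widget.
; Every tick, it re-orients its widget along the look-at rotation from the level's CameraActor to the widget.
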(event `Travel`
  (`/Engine/EditorBlueprintResources/ActorMacros.Switch Has Authority`
    (:`Authority`
      (`AdvancedSessionsLibrary.ServerTravel` "LVL_MiniMap"))))

(event `self.ReceiveTick`
  (params (DeltaSeconds :type "Float (single-precision)"))
  (`self.UpdateWidgetRotation`))

(event `Serv_SetSteamInfos`
  (`self.Mult_SetSteamInfos`))

(event `Mult_SetSteamInfos`
  (for _array_element (`GameStateBase.PlayerArray` (cast `CustomGameState` (`GameplayStatics.GetGameState`) :!pure true))
    (bind _asbp_lobby_player (cast `/Game/Core/Blueprints/Lobby/BP_LobbyPlayer` (`PlayerState.GetPawn` _array_element)))
    (bind _aswbp_steam_informations (cast `/Game/Core/Blueprints/Lobby/WBP_SteamInformations` (`WidgetComponent.GetWidget` (`/Game/Core/Blueprints/Lobby/BP_LobbyPlayer.Widget` _asbp_lobby_player))))
    (bind _uniquenetid (`AdvancedSessionsLibrary.GetUniqueNetIDFromPlayerState` _array_element))
    (bind _returnvalue (`AdvancedSteamFriendsLibrary.GetSteamPersonaName` _uniquenetid))
    (`TextBlock.SetText` (`/Game/Core/Blueprints/Lobby/WBP_SteamInformations.Text_Username` _aswbp_steam_informations) (`KismetTextLibrary.Conv_StringToText` _returnvalue))
    (bind _returnvalue_2 (`AdvancedSteamFriendsLibrary.GetSteamFriendAvatar` _uniquenetid)
      (:`OnSuccess`
        _)
      (:`AsyncLoading`
        _))
    (`Image.SetBrushFromTexture` (`/Game/Core/Blueprints/Lobby/WBP_SteamInformations.Image_Avatar` _aswbp_steam_informations) _returnvalue_2 false)))

(fn `UpdateWidgetRotation`
  (bind _returnvalue (`GameplayStatics.GetActorOfClass` "/Script/Engine.CameraActor"))
  (`/Engine/EditorBlueprintResources/StandardMacros.IsValid` _returnvalue
    (:`Is Valid`
      (bind (_returnvalue_roll _returnvalue_pitch _returnvalue_yaw) (`KismetMathLibrary.BreakRotator` (`KismetMathLibrary.FindLookAtRotation` (`self.K2_GetActorLocation` _returnvalue) (`SceneComponent.K2_GetComponentLocation` (`self.Widget`)))))
      (`SceneComponent.K2_SetWorldRotation` (`self.Widget`) (`KismetMathLibrary.MakeRotator` _returnvalue_roll _returnvalue_pitch _returnvalue_yaw) false false))))

(fn `UserConstructionScript`)