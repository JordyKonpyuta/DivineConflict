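; Lobby player controller that sets up the lobby UI, camera view and character meshes.
; BeginPlay creates the lobby widget for the local controller and routes mesh setup through S_HandleMesh to OC_HandleLobbyMesh, which assigns each player's pawn mesh by PlayerArray index.
; OC_HandleLogin waits briefly, switches the view to a level CameraActor and has the new player's BP_LobbyPlayer set its Steam info.
; A separate event shows the loading screen widget.
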(event `self.ReceiveBeginPlay`
  ;[1 1 1] Begin Play
  (`self.S_HandleMesh`)
  (if (`self.IsLocalPlayerController`)
    (bind _returnvalue (`|CreateWidget` "/Game/Core/Blueprints/Lobby/WBP_Lobby.WBP_Lobby_C"))
    (`UserWidget.AddToViewport` _returnvalue 0)))

(event `OC_HandleLogin`
  (params (NewPlayer :type "/Game/Core/Blueprints/Lobby/PC_Lobby Object Reference"))
  ;[1 1 1] On login event
  (`KismetSystemLibrary.Delay` 0.5)
  (bind _returnvalue (`GameplayStatics.GetActorOfClass` "/Script/Engine.CameraActor"))
  (`self.SetViewTargetWithBlend` _returnvalue)
  (bind _asbp_lobby_player (cast `/Game/Core/Blueprints/Lobby/BP_LobbyPlayer` (`self.K2_GetPawn` NewPlayer)))
  (`/Game/Core/Blueprints/Lobby/BP_LobbyPlayer.Serv_SetSteamInfos` _asbp_lobby_player))

(event `OC_LoadingScreen`
  ;[1 1 1] Loading Screen
  (bind _returnvalue (`|CreateWidget` "/Game/Core/Blueprints/Widget/WBP_LoadingScreen.WBP_LoadingScreen_C"))
  (`UserWidget.AddToViewport` _returnvalue 0))

(event `OC_HandleLobbyMesh`
  ;[1 1 1] Handle Lobby Mesh
  (for (_array_element _array_index) (`GameStateBase.PlayerArray` (`GameplayStatics.GetGameState`))
    (bind _asbp_lobby_player (cast `/Game/Core/Blueprints/Lobby/BP_LobbyPlayer` (`PlayerState.GetPawn` _array_element)))
    (`StaticMeshComponent.SetStaticMesh` (`/Game/Core/Blueprints/Lobby/BP_LobbyPlayer.StaticMesh` _asbp_lobby_player) (select `int` _array_index :`0` "/Game/Game_Art/Asset_temp/Character/Paradis/Chara_Ange_test_Shape.Chara_Ange_test_Shape" :`1` "/Game/Game_Art/Asset_temp/Character/enfer/chara_guerrier/guerrier01.guerrier01" :!type "StaticMesh Object Reference"))))

(event `S_HandleMesh`
  ;[1 1 1] Handle Lobby Mesh
  (`self.OC_HandleLobbyMesh`))

(fn `UserConstructionScript`)