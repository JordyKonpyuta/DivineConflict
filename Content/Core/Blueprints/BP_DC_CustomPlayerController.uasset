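; Player controller for a turn-based game with units and buildings, acting as the hub for the local player's UI.
; On BeginPlay it creates the HUD, or views a CameraActor in the main menu.
; Display events push unit, building, base, tower, attack, pause and end-level widgets onto HUD stacks.
; Other events refresh player info and turn timer or drive the camera's interaction widget, while the change-turn input is empty.
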(event `self.ReceiveBeginPlay`
  ;[1 1 1] Begin Play
  (if (`self.IsLocalController`)
    (if (not (`self.IsInMainMenu`))
      (bind _returnvalue (`|CreateWidget` "/Game/Core/Blueprints/Widget/HUD/WBP_HUD.WBP_HUD_C"))
      (bind _output_get (set `self.WBP_HUD_Ref` _returnvalue))
      (`UserWidget.AddToViewport` _output_get 0)
      (else
        (bind _returnvalue_2 (`GameplayStatics.GetActorOfClass` "/Script/Engine.CameraActor"))
        (`self.SetViewTargetWithBlend` _returnvalue_2)))))

(event `self.RemoveAttackWidget`
  (bind _wbp_hud_ref (`self.WBP_HUD_Ref`))
  ;[0.5245 0.7717 1] Widget Displaying
  ;;[1 1 1] Remove Attack widget
  (bind _wbp_feedback_attack (`self.WBP Feedback Attack`)
    (:`then`
      (`/Game/Core/Blueprints/Widget/HUD/WBP_HUD.RemoveWidget` _wbp_hud_ref (`/Game/Core/Blueprints/Widget/HUD/WBP_HUD.WidgetStack_Builds` _wbp_hud_ref) _wbp_feedback_attack))
    (:`else`)))

(event `self.DisplayWidget`
  (bind _wbp_hud_ref (`self.WBP_HUD_Ref`))
  ;[0.5245 0.7717 1] Widget Displaying
  ;;[1 1 1] Units Widget
  (`/Game/Core/Blueprints/Widget/HUD/WBP_HUD.PushWidget` _wbp_hud_ref (`/Game/Core/Blueprints/Widget/HUD/WBP_HUD.WidgetStack_Unit` _wbp_hud_ref) "/Game/Core/Blueprints/Widget/HUD/WBP_Units.WBP_Units_C"))

(event `self.HiddeWidget`
  ;[0.5245 0.7717 1] Widget Displaying
  (`KismetSystemLibrary.PrintString` "hidden"))

(event `self.DisplayAttackWidget`
  (bind _wbp_hud_ref (`self.WBP_HUD_Ref`))
  ;[0.5245 0.7717 1] Widget Displaying
  ;;[1 1 1] Attack widget
  (`/Game/Core/Blueprints/Widget/HUD/WBP_HUD.PushWidget` _wbp_hud_ref (`/Game/Core/Blueprints/Widget/HUD/WBP_HUD.WidgetStack_Builds` _wbp_hud_ref) "/Game/Core/Blueprints/Widget/HUD/WBP_FeedbackAttack.WBP_FeedbackAttack_C")
  (bind _aswbp_feedback_attack (cast `/Game/Core/Blueprints/Widget/HUD/WBP_FeedbackAttack` (`/Game/Core/Blueprints/Widget/HUD/WBP_HUD.PushedWidget` _wbp_hud_ref)))
  (set `self.WBP Feedback Attack` _aswbp_feedback_attack))

(event `self.DisplayWidgetBuilding`
  (bind _wbp_hud_ref (`self.WBP_HUD_Ref`))
  ;[0.5245 0.7717 1] Widget Displaying
  ;;[1 1 1] Buildings Widget
  (`/Game/Core/Blueprints/Widget/HUD/WBP_HUD.PushWidget` _wbp_hud_ref (`/Game/Core/Blueprints/Widget/HUD/WBP_HUD.WidgetStack_Builds` _wbp_hud_ref) (select `bool` (`|EnumEquality` (`Building.BuildingList` (`self.BuildingRef`)) "B_AP") :`false` "/Game/Core/Blueprints/Widget/HUD/WBP_Builds_New.WBP_Builds_New_C" :`true` "/Game/Core/Blueprints/Widget/HUD/WBP_BuildAP.WBP_BuildAP_C" :!type "CommonActivatableWidget Class Reference")))

(event `EnhancedInput|/Game/Core/Controller/Inputs/IA_ChangeTurn`
  (params (ActionValue :type Boolean) (ElapsedSeconds :type "Float (double-precision)") (TriggeredSeconds :type "Float (double-precision)") (InputAction :type "InputAction Object Reference" :default "/Game/Core/Controller/Inputs/IA_ChangeTurn.IA_ChangeTurn"))
  ;[0.3604 1 0.605] Inputs
  ;;[1 1 1] Change Turn Input
)

(event `self.UpdateUi`
  ;[0.5245 0.7717 1] Widget Displaying
  ;;[1 1 1] Update UI Event
  (if (`self.IsLocalPlayerController`)
    (`/Game/Core/Blueprints/Widget/HUD/WBP_HUD_Paradise.SetPlayerInfos` (`self.WBP_HUD_ParadiseRef`))))

(event `self.DisplayWidgetBase`
  (bind _wbp_hud_ref (`self.WBP_HUD_Ref`))
  ;[0.5245 0.7717 1] Widget Displaying
  ;;[1 1 1] Base Widget
  (`/Game/Core/Blueprints/Widget/HUD/WBP_HUD.PushWidget` _wbp_hud_ref (`/Game/Core/Blueprints/Widget/HUD/WBP_HUD.WidgetStack_Builds` _wbp_hud_ref) "/Game/Core/Blueprints/Widget/HUD/WBP_Base_New.WBP_Base_New_C"))

(event `EnhancedInput|/Game/Core/Controller/Inputs/IA_Pause`
  (params (ActionValue :type Boolean) (ElapsedSeconds :type "Float (double-precision)") (TriggeredSeconds :type "Float (double-precision)") (InputAction :type "InputAction Object Reference" :default "/Game/Core/Controller/Inputs/IA_Pause.IA_Pause"))
  (bind _wbp_hud_ref (`self.WBP_HUD_Ref`))
  ;[0.3604 1 0.605] Inputs
  ;;[1 1 1] "Pause" Input
  (:`Started`
    (`/Game/Core/Blueprints/Widget/HUD/WBP_HUD.PushWidget` _wbp_hud_ref (`/Game/Core/Blueprints/Widget/HUD/WBP_HUD.WidgetStack_HUD` _wbp_hud_ref) "/Game/Core/Blueprints/Widget/HUD/WBP_Pause_Paradise.WBP_Pause_Paradise_C")
    (bind _aswbp_pause_paradise (cast `/Game/Core/Blueprints/Widget/HUD/WBP_Pause_Paradise` (`/Game/Core/Blueprints/Widget/HUD/WBP_HUD.PushedWidget` _wbp_hud_ref)))
    (set `/Game/Core/Blueprints/Widget/HUD/WBP_Pause_Paradise.HUD_Ref` (`self.WBP_HUD_Ref`) _aswbp_pause_paradise)))

(event `self.UpdateUITimer`
  (params (TimeLeft :type Integer))
  (bind _wbp_hud_paradiseref (`self.WBP_HUD_ParadiseRef`))
  ;[0.5245 0.7717 1] Widget Displaying
  ;;[1 1 1] Update UI Timer
  (`/Engine/EditorBlueprintResources/StandardMacros.IsValid` _wbp_hud_paradiseref
    (:`Is Valid`
      (set `/Game/Core/Blueprints/Widget/HUD/WBP_HUD_Paradise.Timer` TimeLeft _wbp_hud_paradiseref)
      (`/Game/Core/Blueprints/Widget/HUD/WBP_HUD_Paradise.PlayTurnAnimation` _wbp_hud_paradiseref))))

(event `self.DisplayWidgetTower`
  (bind _wbp_hud_ref (`self.WBP_HUD_Ref`))
  ;[0.5245 0.7717 1] Widget Displaying
  ;;[1 1 1] Tower Widget
  (`/Game/Core/Blueprints/Widget/HUD/WBP_HUD.PushWidget` _wbp_hud_ref (`/Game/Core/Blueprints/Widget/HUD/WBP_HUD.WidgetStack_Builds` _wbp_hud_ref) "/Game/Core/Blueprints/Widget/HUD/WBP_Tower_New.WBP_Tower_New_C"))

(event `self.UpdateWidget3D`
  (params (Index :type Integer) (bVisibility :type Boolean))
  ;[0.5245 0.7717 1] Widget Displaying
  ;;[1 1 1] Update Widget 3D
  (bind _asbp_dc_camera_player (cast `/Game/Core/Blueprints/BP_DC_CameraPlayer` (`self.CameraPlayerRef`)))
  (`|ExecutionSequence`
    (:`then_0`
      (bind _widget (`/Game/Core/Blueprints/BP_DC_CameraPlayer.Widget` _asbp_dc_camera_player))
      (bind _aswbp_interaction (cast `/Game/Core/Blueprints/Widget/WBP_Interaction` (`WidgetComponent.GetWidget` _widget)))
      (`WidgetSwitcher.SetActiveWidgetIndex` (`/Game/Core/Blueprints/Widget/WBP_Interaction.WidgetSwitcher` _aswbp_interaction) Index))
    (:`then_1`
      (`SceneComponent.SetVisibility` _widget bVisibility false))))

(event `DisplayEndLevel`
  (bind _wbp_hud_ref (`self.WBP_HUD_Ref`))
  ;[0.5245 0.7717 1] Widget Displaying
  ;;[1 1 1] Display End Level UI
  (`/Game/Core/Blueprints/Widget/HUD/WBP_HUD.PushWidget` _wbp_hud_ref (`/Game/Core/Blueprints/Widget/HUD/WBP_HUD.WidgetStack_HUD` _wbp_hud_ref) "/Game/Core/Blueprints/Widget/HUD/WBP_EndLevel.WBP_EndLevel_C"))

(fn `UserConstructionScript`)