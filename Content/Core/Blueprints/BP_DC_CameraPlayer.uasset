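; BP_DC_CameraPlayer is a camera player Blueprint with a follow camera and a widget component that is turned toward that camera.
; On BeginPlay it disables the widget's shadow, sets its initial rotation and registers itself as CameraPlayer on BP_CustomGameInstance.
; The RotateWidget event applies the look-at rotation from widget to camera, adding a scaled yaw offset from ValueX and a pitch offset from ValueY.
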(event `self.ReceiveBeginPlay`
  (`PrimitiveComponent.SetCastShadow` (`self.Widget`) false)
  (`self.RotateWidget` 0.0)
  (set `CustomGameInstance.CameraPlayer` self (cast `/Game/Core/BP_CustomGameInstance` (`GameplayStatics.GetGameInstance`) :!pure true)))

(event `self.RotateWidget`
  (params (ValueX :type "Float (single-precision)") (ValueY :type "Float (single-precision)"))
  (bind _widget (`self.Widget`))
  (bind (_returnvalue_roll _returnvalue_pitch _returnvalue_yaw) (`KismetMathLibrary.BreakRotator` (`KismetMathLibrary.FindLookAtRotation` (`SceneComponent.K2_GetComponentLocation` _widget) (`SceneComponent.K2_GetComponentLocation` (`self.FollowCamera`)))))
  (`SceneComponent.K2_SetWorldRotation` _widget (`KismetMathLibrary.MakeRotator` _returnvalue_roll (+ ValueY _returnvalue_pitch) (+ (* ValueX -90.0) _returnvalue_yaw)) false false))

(fn `UserConstructionScript`)