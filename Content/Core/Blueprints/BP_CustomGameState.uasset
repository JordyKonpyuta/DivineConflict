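; Custom game state for a two-player game, handling lobby start checks and end-of-level results.
; It tells the first player's lobby controller whether the game can launch, based on having at least two players.
; It triggers the end-level display on each player's controller.
; SetVictoryScreenInfos returns winner and loser Steam names and avatars, falling back to numbered player names and a chess pawn image.
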(event `self.DisplayWidget`
  (for _array_element (`self.PlayerArray`)
    (bind _asbp_dc_custom_player_controller (cast `/Game/Core/Blueprints/BP_DC_CustomPlayerController` (`PlayerState.GetPlayerController` _array_element)))
    (`/Game/Core/Blueprints/BP_DC_CustomPlayerController.DisplayEndLevel` _asbp_dc_custom_player_controller)))

(event `CheckCanStartGameLobby`
  (bind _returnvalue (`PlayerState.GetPlayerController` (`GameplayStatics.GetPlayerState` 0)))
  (if (>= (`KismetArrayLibrary.Array_Length` (`self.PlayerArray`)) 2)
    (bind _aspc_lobby (cast `/Game/Core/Blueprints/Lobby/PC_Lobby` _returnvalue))
    (`/Game/Core/Blueprints/Lobby/PC_Lobby.Serv_CanLaunchGame` _aspc_lobby)
    (else
      (bind _aspc_lobby_2 (cast `/Game/Core/Blueprints/Lobby/PC_Lobby` _returnvalue))
      (`/Game/Core/Blueprints/Lobby/PC_Lobby.Serv_CantLaunchGame` _aspc_lobby_2))))

(fn `SetVictoryScreenInfos`
  (returns (UsernameWinner :type String) (UsernameLoser :type String) (AvatarWinner :type "Texture2D Object Reference") (AvatarLoser :type "Texture2D Object Reference"))
  (bind _uniquenetid (`AdvancedSessionsLibrary.GetUniqueNetIDFromPlayerState` (`self.PLoser`)))
  (bind _uniquenetid_2 (`AdvancedSessionsLibrary.GetUniqueNetIDFromPlayerState` (`self.PWinner`)))
  (`|ExecutionSequence`
    (:`then_0`
      (bind _returnvalue (`AdvancedSteamFriendsLibrary.GetSteamPersonaName` _uniquenetid))
      (if (not (`KismetStringLibrary.IsEmpty` _returnvalue))
        (set `self.UsernameLoser` _returnvalue)
        (bind _returnvalue_2 (`AdvancedSteamFriendsLibrary.GetSteamFriendAvatar` _uniquenetid)
          (:`OnSuccess`
            _)
          (:`AsyncLoading`
            _))
        (set `self.AvatarLoser` _returnvalue_2)
        (else
          (set `self.UsernameLoser` (`KismetStringLibrary.Concat_StrStr` "Player " (select `bool` (== (`self.PLoser`) (`|GetArrayItem` (`self.PlayerArray`))) :`false` "2" :`true` "1")))
          (set `self.AvatarLoser` "/Game/Icons/chess_piece_pawn.chess_piece_pawn"))))
    (:`then_1`
      (bind _returnvalue_3 (`AdvancedSteamFriendsLibrary.GetSteamPersonaName` _uniquenetid_2))
      (if (not (`KismetStringLibrary.IsEmpty` _returnvalue_3))
        (set `self.UsernameWinner` _returnvalue_3)
        (bind _returnvalue_4 (`AdvancedSteamFriendsLibrary.GetSteamFriendAvatar` _uniquenetid_2)
          (:`OnSuccess`
            _)
          (:`AsyncLoading`
            _))
        (set `self.AvatarWinner` _returnvalue_4)
        (else
          (set `self.UsernameWinner` (`KismetStringLibrary.Concat_StrStr` "Player " (select `bool` (== (`|GetArrayItem` (`self.PlayerArray`)) (`self.PWinner`)) :`false` "2" :`true` "1")))
          (set `self.AvatarWinner` "/Game/Icons/chess_piece_pawn.chess_piece_pawn"))))
    (:`then_2`
      (return (`self.UsernameWinner`) (`self.UsernameLoser`) (`self.AvatarWinner`) (`self.AvatarLoser`)))))

(fn `UserConstructionScript`)