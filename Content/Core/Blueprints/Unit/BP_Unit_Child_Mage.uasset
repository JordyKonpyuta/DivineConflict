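; BP_Unit_Child_Mage is the Mage unit Blueprint, defining how that unit's stats are loaded and reset.
; SetStats copies current health, max health, attack, defense and PM from its DataAsset through the unit's setters.
; SetDefaultStats writes hardcoded Mage values directly into that DataAsset, so the defaults live in this Blueprint and modify the asset itself rather than the unit's variables.
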(fn `SetDefaultStats`
  (bind _dataasset (`self.DataAsset`))
  (set `/Game/Core/Tool/DataAsset/PDA_UnitsStats.CurrentHealth` 10 _dataasset)
  (set `/Game/Core/Tool/DataAsset/PDA_UnitsStats.MaxHealth` 10 _dataasset)
  (set `/Game/Core/Tool/DataAsset/PDA_UnitsStats.Attack` 5 _dataasset)
  (set `/Game/Core/Tool/DataAsset/PDA_UnitsStats.Defense` 2 _dataasset)
  (set `/Game/Core/Tool/DataAsset/PDA_UnitsStats.PM` 4 _dataasset))

(fn `SetStats`
  (bind _dataasset (`self.DataAsset`))
  (`self.SetCurrentHealth` (`/Game/Core/Tool/DataAsset/PDA_UnitsStats.CurrentHealth` _dataasset))
  (`self.SetMaxHealth` (`/Game/Core/Tool/DataAsset/PDA_UnitsStats.MaxHealth` _dataasset))
  (`self.SetAttack` (`/Game/Core/Tool/DataAsset/PDA_UnitsStats.Attack` _dataasset))
  (`self.SetDefense` (`/Game/Core/Tool/DataAsset/PDA_UnitsStats.Defense` _dataasset))
  (`self.SetPM` (`/Game/Core/Tool/DataAsset/PDA_UnitsStats.PM` _dataasset)))

(fn `UserConstructionScript`)