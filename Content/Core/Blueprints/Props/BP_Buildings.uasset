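; BP_Buildings is a configurable prop for resource buildings, with Wood, Stone, Gold and AP variants.
; Its construction script switches on the BuildingList enum to set the building mesh, with a Hell flag choosing between meshes for Wood, Stone and Gold.
; It also assigns a plane mesh beneath the same switch, scaled larger for AP, which ignores Hell.
; The event graph holds no active logic.
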(fn `UserConstructionScript`
  (bind _staticmeshplane (`self.StaticMeshPlane`))
  (bind _staticmeshplane_2 (`self.StaticMeshPlane`))
  (bind _staticmeshbuilding (`self.StaticMeshBuilding`))
  (switch `EBuildingList` (`self.BuildingList`)
    (:`B_Wood`
      (`StaticMeshComponent.SetStaticMesh` _staticmeshbuilding (select `bool` (`self.Hell`) :`false` "/Game/Game_Art/Assets/pin.pin" :!type "StaticMesh Object Reference"))
      (`StaticMeshComponent.SetStaticMesh` _staticmeshplane "/Engine/BasicShapes/Plane.Plane" :!label _label)
      (`SceneComponent.SetRelativeScale3D` _staticmeshplane (2.0 2.0 2.0)))
    (:`B_Stone`
      (`StaticMeshComponent.SetStaticMesh` _staticmeshbuilding (select `bool` (`self.Hell`) :`false` "/Game/Game_Art/Asset_temp/Rock/Rock_group_low.Rock_group_low" :!type "StaticMesh Object Reference"))
      (goto _label))
    (:`B_Gold`
      (`StaticMeshComponent.SetStaticMesh` _staticmeshbuilding (select `bool` (`self.Hell`) :`false` "/Game/Game_Art/Assets/SM_Buisson.SM_Buisson" :!type "StaticMesh Object Reference"))
      (goto _label))
    (:`B_AP`
      (`StaticMeshComponent.SetStaticMesh` _staticmeshbuilding "/Engine/BasicShapes/Cone.Cone")
      (`StaticMeshComponent.SetStaticMesh` _staticmeshplane_2 "/Engine/BasicShapes/Plane.Plane")
      (`SceneComponent.SetRelativeScale3D` _staticmeshplane_2 (3.0 3.0 3.0)))))