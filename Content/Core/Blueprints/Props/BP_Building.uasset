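; Building prop for resource farms (Wood, Stone, Gold) and the central AP building, with visuals set by type and owning faction.
; The construction script switches on BuildingList and selects skeletal mesh and animation by PlayerOwner (Hell or Heaven, Neutral left empty), though some assets are shared or cross-faction.
; AP ignores owner, using one rotated mesh and a larger base plane.
; StaticMeshBuilding is skeletal despite its name, and the event graph has no logic.
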(fn `UserConstructionScript`
  (bind _staticmeshplane (`self.StaticMeshPlane`))
  (bind _playerowner (`self.PlayerOwner`))
  (bind _playerowner_2 (`self.PlayerOwner`))
  (bind _playerowner_3 (`self.PlayerOwner`))
  (bind _staticmeshplane_2 (`self.StaticMeshPlane`))
  (bind _staticmeshbuilding (`self.StaticMeshBuilding`))
  (switch `EBuildingList` (`self.BuildingList`)
    (:`B_Wood`
      (`SkeletalMeshComponent.SetSkeletalMeshAsset` _staticmeshbuilding (select `EPlayer` _playerowner :`P_Hell` "/Game/Game_Art/Assets/Farm/Wood/Paradise/Farm_Wood_Paradise.Farm_Wood_Paradise" :`P_Heaven` "/Game/Game_Art/Assets/Farm/Wood/Paradise/Farm_Wood_Paradise.Farm_Wood_Paradise" :!type "SkeletalMesh Object Reference"))
      (set `SkeletalMeshComponent.AnimationData` (make `SingleAnimationPlayData` :`AnimToPlay` (select `EPlayer` _playerowner :`P_Hell` "/Game/Game_Art/Assets/Farm/Wood/Hell/Farm_Wood_Hell_Anim.Farm_Wood_Hell_Anim" :`P_Heaven` "/Game/Game_Art/Assets/Farm/Wood/Paradise/Farm_Wood_Paradise_Anim.Farm_Wood_Paradise_Anim" :!type "AnimationAsset Object Reference")) (`self.StaticMeshBuilding`))
      (`StaticMeshComponent.SetStaticMesh` _staticmeshplane "/Engine/BasicShapes/Plane.Plane" :!label _label)
      (`SceneComponent.SetRelativeScale3D` _staticmeshplane (2.0 2.0 2.0)))
    (:`B_Stone`
      (`SkeletalMeshComponent.SetSkeletalMeshAsset` _staticmeshbuilding (select `EPlayer` _playerowner_2 :`P_Hell` "/Game/Game_Art/Assets/Farm/Stone/Paradise/Farm_Stone_Paradise.Farm_Stone_Paradise" :`P_Heaven` "/Game/Game_Art/Assets/Farm/Stone/Hell/SKM_Farm_Stone_Hell.SKM_Farm_Stone_Hell" :!type "SkeletalMesh Object Reference"))
      (set `SkeletalMeshComponent.AnimationData` (make `SingleAnimationPlayData` :`AnimToPlay` (select `EPlayer` _playerowner_2 :`P_Hell` "/Game/Game_Art/Assets/Farm/Stone/Hell/AS_Farm_Stone_Hell.AS_Farm_Stone_Hell" :`P_Heaven` "/Game/Game_Art/Assets/Farm/Stone/Paradise/Farm_Stone_Paradise_Anim.Farm_Stone_Paradise_Anim" :!type "AnimationAsset Object Reference")) (`self.StaticMeshBuilding`))
      (goto _label))
    (:`B_Gold`
      (`SkeletalMeshComponent.SetSkeletalMeshAsset` _staticmeshbuilding (select `EPlayer` _playerowner_3 :`P_Hell` "/Game/Game_Art/Assets/Farm/Gold/SKM_Farm_Gold_Hell.SKM_Farm_Gold_Hell" :`P_Heaven` "/Game/Game_Art/Assets/Farm/Gold/SKM_Farm_Gold_Hell.SKM_Farm_Gold_Hell" :!type "SkeletalMesh Object Reference"))
      (set `SkeletalMeshComponent.AnimationData` (make `SingleAnimationPlayData` :`AnimToPlay` (select `EPlayer` _playerowner_3 :`P_Hell` "/Game/Game_Art/Assets/Farm/Gold/AS_Farm_Gold_Hell.AS_Farm_Gold_Hell" :`P_Heaven` "/Game/Game_Art/Assets/Farm/Gold/AS_Farm_Gold_Hell.AS_Farm_Gold_Hell" :!type "AnimationAsset Object Reference")) (`self.StaticMeshBuilding`))
      (goto _label))
    (:`B_AP`
      (`SkeletalMeshComponent.SetSkeletalMeshAsset` _staticmeshbuilding "/Game/Game_Art/Assets/Farm/PA/Farm_PA_Central.Farm_PA_Central")
      (`SceneComponent.K2_SetWorldRotation` (`self.StaticMeshBuilding`) (struct :`Yaw` -45.0) false false)
      (set `SkeletalMeshComponent.AnimationData` (make `SingleAnimationPlayData` :`AnimToPlay` "/Game/Game_Art/Assets/Farm/PA/Farm_PA_Central_Anim.Farm_PA_Central_Anim") (`self.StaticMeshBuilding`))
      (`StaticMeshComponent.SetStaticMesh` _staticmeshplane_2 "/Engine/BasicShapes/Plane.Plane")
      (`SceneComponent.SetRelativeScale3D` _staticmeshplane_2 (3.0 3.0 3.0)))))