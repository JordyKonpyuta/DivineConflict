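; Custom player controller that turns directional input into wrap-around index navigation for UI focus.
; On BeginPlay it adds the UI navigation mapping context to the Enhanced Input subsystem of player 0.
; Up/Down and Left/Right actions step separate vertical and horizontal indices, both wrapping between zero and a shared MaxIndex.
; Each step fires the UpdateFocus event dispatcher, leaving the actual focus change to its listeners.
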(event `self.ReceiveBeginPlay`
  ;[1 1 1] Event Construct
  (`EnhancedInputSubsystemInterface.AddMappingContext` (pcsubsystem `EnhancedInputLocalPlayerSubsystem` (`GameplayStatics.GetPlayerController` 0)) "/Game/Core/Controller/IMC_UINavigation.IMC_UINavigation" 0 (struct)))

(event `EnhancedInput|/Game/Core/Controller/Inputs/UI_Navigation/IA_Up`
  (params (ActionValue :type Boolean) (ElapsedSeconds :type "Float (double-precision)") (TriggeredSeconds :type "Float (double-precision)") (InputAction :type "InputAction Object Reference" :default "/Game/Core/Controller/Inputs/UI_Navigation/IA_Up.IA_Up"))
  ;[1 1 1] UI Navigation : Up and Down
  (:`Triggered`
    (if (> (`self.VerticalIndex`) 0)
      (`/Engine/EditorBlueprintResources/StandardMacros.DecrementInt` (`self.VerticalIndex`)
        (:`  `
          _))
      (else
        (set `self.VerticalIndex` (`self.MaxIndex`))))
    (`self.ED_UpdateFocus`)))

(event `EnhancedInput|/Game/Core/Controller/Inputs/UI_Navigation/IA_Left`
  (params (ActionValue :type Boolean) (ElapsedSeconds :type "Float (double-precision)") (TriggeredSeconds :type "Float (double-precision)") (InputAction :type "InputAction Object Reference" :default "/Game/Core/Controller/Inputs/UI_Navigation/IA_Left.IA_Left"))
  ;[1 1 1] UI Navigation : Left and Right
  (:`Triggered`
    (if (> (`self.HorizontalIndex`) 0)
      (`/Engine/EditorBlueprintResources/StandardMacros.DecrementInt` (`self.HorizontalIndex`)
        (:`  `
          _))
      (else
        (set `self.HorizontalIndex` (`self.MaxIndex`))))
    (`self.ED_UpdateFocus`)))

(event `EnhancedInput|/Game/Core/Controller/Inputs/UI_Navigation/IA_Down`
  (params (ActionValue :type Boolean) (ElapsedSeconds :type "Float (double-precision)") (TriggeredSeconds :type "Float (double-precision)") (InputAction :type "InputAction Object Reference" :default "/Game/Core/Controller/Inputs/UI_Navigation/IA_Down.IA_Down"))
  ;[1 1 1] UI Navigation : Up and Down
  (:`Triggered`
    (if (< (`self.VerticalIndex`) (`self.MaxIndex`))
      (`/Engine/EditorBlueprintResources/StandardMacros.IncrementInt` (`self.VerticalIndex`)
        (:`  `
          _))
      (else
        (set `self.VerticalIndex` 0)))
    (`self.ED_UpdateFocus`)))

(event `EnhancedInput|/Game/Core/Controller/Inputs/UI_Navigation/IA_Right`
  (params (ActionValue :type Boolean) (ElapsedSeconds :type "Float (double-precision)") (TriggeredSeconds :type "Float (double-precision)") (InputAction :type "InputAction Object Reference" :default "/Game/Core/Controller/Inputs/UI_Navigation/IA_Right.IA_Right"))
  ;[1 1 1] UI Navigation : Left and Right
  (:`Triggered`
    (if (< (`self.HorizontalIndex`) (`self.MaxIndex`))
      (`/Engine/EditorBlueprintResources/StandardMacros.IncrementInt` (`self.HorizontalIndex`)
        (:`  `
          _))
      (else
        (set `self.HorizontalIndex` 0)))
    (`self.ED_UpdateFocus`)))

(fn `UserConstructionScript`)