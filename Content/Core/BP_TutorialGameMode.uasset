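; Tutorial game mode that teaches the tactics game in nine lessons, from movement and production to unit skills, capture and victory conditions.
; BeginTutorial shows a timed loading screen, then calls DisplayTutorialWidget, which maps an index to a lesson event and highlights the relevant unit for some.
; Each lesson calls InitUI to push WBP_Tutorial onto the player controller's HUD stack, fills its hardcoded lines and also adds it to the viewport.
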(event `self.BeginTutorial`
  ;[1 1 1] Begin Play
  (bind _returnvalue (`|CreateWidget` "/Game/Core/Blueprints/Widget/WBP_LoadingScreen.WBP_LoadingScreen_C"))
  (`UserWidget.AddToViewport` _returnvalue 0)
  (`KismetSystemLibrary.Delay` 2.0)
  (`Widget.RemoveFromParent` _returnvalue)
  (`self.DisplayTutorialWidget` 0))

(event `MovingAttackElevate`
  (bind _ui_tutorialref (`self.UI_TutorialRef`))
  ;[1 1 1] Set Tutorial Lines on widget
  (`self.InitUI`)
  (set `/Game/Core/Blueprints/Widget/Tutorial/WBP_Tutorial.TutorialLines` (`|MakeArray` "We're going to talk about three things here: moving, attacking and ending a turn." "First of all, moving. Once you've selected a unit and chosen the move option, you can decide which route it will take. A ghost will appear at its final destination to warn you." "Next, the attack. A unit may attack an adjacent square once per turn. If it is on a half-square higher than its target, it will inflict more damage." "Once you've made your choice, press START to execute your orders." "Note: the tank has just enough HP to survive an attack by the warrior on even ground." "Solution: the warrior must be placed high up to eliminate the tank." :!type "Text") _ui_tutorialref)
  (`UserWidget.AddToViewport` _ui_tutorialref 0))

(event `MageAbility`
  (bind _ui_tutorialref (`self.UI_TutorialRef`))
  ;[1 1 1] Set Tutorial Lines on widget
  (`self.InitUI`)
  (set `/Game/Core/Blueprints/Widget/Tutorial/WBP_Tutorial.TutorialLines` (`|MakeArray` "Let's talk about skills, starting with the mage." "Each unit has a skill it can use once per turn, at a cost of APs." "The mage's skill allows him to inflict damage from two squares away, ignoring enemy defense. What's more, this skill has a longer range if used on a ledge." "Note: the warrior has just enough HP to die after two mage skills." "Solution: each mage must use his skill. The high mage gains 1 range on the ledge." :!type "Text") _ui_tutorialref)
  (`UserWidget.AddToViewport` _ui_tutorialref 0))

(event `CityCapture`
  (bind _ui_tutorialref (`self.UI_TutorialRef`))
  ;[1 1 1] Set Tutorial Lines on widget
  (`self.InitUI`)
  (set `/Game/Core/Blueprints/Widget/Tutorial/WBP_Tutorial.TutorialLines` (`|MakeArray` "Buildings start out neutral, but can be controlled by either player. Once controlled, they offer several advantages." "To take control of a building, a unit must be placed on it, which becomes the city's garrison." "If an enemy garrison is already present in a building, it must be eliminated before the building can be taken." "The building in front of your warrior is empty. Take control of it." "Solution: the warrior must garrison the town." :!type "Text") _ui_tutorialref)
  (`UserWidget.AddToViewport` _ui_tutorialref 0))

(event `self.DisplayTutorialWidget`
  (params (index :type Integer))
  ;[1 1 1] Display Widget Tutorial
  (switch `int` index
    (:`0`
      (`self.MovingAttackElevate`)
      (`self.HilightUnit` (`self.Tank`)))
    (:`1`
      (`self.BaseProduction`))
    (:`2`
      (`self.MageAbility`)
      (`self.HilightUnit` (`self.Warrior1`)))
    (:`3`
      (`self.WarriorAbility`)
      (`self.HilightUnit` (`self.Mage`)))
    (:`4`
      (`self.TankAbility`)
      (`self.HilightUnit` (`self.Warrior2`)))
    (:`5`
      (`self.LeaderPassive`)
      (`self.HilightUnit` (`self.Leader`)))
    (:`6`
      (`self.CityCapture`))
    (:`7`
      (`self.CityProduction`))
    (:`8`
      (`self.VictoryConditions`))))

(event `WarriorAbility`
  (bind _ui_tutorialref (`self.UI_TutorialRef`))
  ;[1 1 1] Set Tutorial Lines on widget
  (`self.InitUI`)
  (set `/Game/Core/Blueprints/Widget/Tutorial/WBP_Tutorial.TutorialLines` (`|MakeArray` "The warrior's skill enables him to climb certain marked walls. Use it to eliminate the mage above." "Note: the wall directly in the path is marked. Solution: the warrior must move towards the wall, climb up, then attack." :!type "Text") _ui_tutorialref)
  (`UserWidget.AddToViewport` _ui_tutorialref 0))

(event `CityProduction`
  (bind _ui_tutorialref (`self.UI_TutorialRef`))
  ;[1 1 1] Set Tutorial Lines on widget
  (`self.InitUI`)
  (set `/Game/Core/Blueprints/Widget/Tutorial/WBP_Tutorial.TutorialLines` (`|MakeArray` "Like the main base, the buildings produce resources and units, but are more limited." "Each building can produce only one type of resource, and only one type of unit. For example, the building you control produces wood, and can produce mages." "You're in the production phase, so produce a mage in your new building." "Note: the player only has enough resources to produce one mage. If he produces the mage in the main base, it's a failure." "Solution: produce a mage in the controlled building." :!type "Text") _ui_tutorialref)
  (`UserWidget.AddToViewport` _ui_tutorialref 0))

(event `BaseProduction`
  (bind _ui_tutorialref (`self.UI_TutorialRef`))
  ;[1 1 1] Set Tutorial Lines on widget
  (`self.InitUI`)
  (set `/Game/Core/Blueprints/Widget/Tutorial/WBP_Tutorial.TutorialLines` (`|MakeArray` "After the active turn, where you give orders to your troops, you move on to the production turn, where you choose which units to produce." "In the corner of the map, you can see your base. It produces resources of each type (Gold, Stone and Wood) every turn, and can produce any type of unit." "To produce a unit, select the base, then the chosen unit. Then press START to execute your orders." "Note: the player has enough resources to produce one basic unit, but not 2. Solution: the player simply chooses a unit to produce and finishes his turn." :!type "Text") _ui_tutorialref)
  (`UserWidget.AddToViewport` _ui_tutorialref 0))

(event `TankAbility`
  (bind _ui_tutorialref (`self.UI_TutorialRef`))
  ;[1 1 1] Set Tutorial Lines on widget
  (`self.InitUI`)
  (set `/Game/Core/Blueprints/Widget/Tutorial/WBP_Tutorial.TutorialLines` (`|MakeArray` "The tank's skill allows it to increase the defense of adjacent units for one turn. Use it to eliminate the enemy warrior without losing your own warrior." "Pay attention to the order of the actions." "Note: both warriors have just enough HP to die in a fight against each other." "Solution: both units must move, the tank must use its skill, then the warrior must attack." :!type "Text") _ui_tutorialref)
  (`UserWidget.AddToViewport` _ui_tutorialref 0))

(event `VictoryConditions`
  (bind _ui_tutorialref (`self.UI_TutorialRef`))
  ;[1 1 1] Set Tutorial Lines on widget
  (`self.InitUI`)
  (set `/Game/Core/Blueprints/Widget/Tutorial/WBP_Tutorial.TutorialLines` (`|MakeArray` "Finally, let's talk about your final goal: to destroy the door to your opponent's base." "Each base has a certain number of HP, representing the integrity of its main door." "These HP can be reduced by attacking the door, in the same way as you attack other units." "Your aim is to reduce the enemy base's HP to 0, while protecting your own base. Use your three units to finish this battle." "Note: the opposing base has just enough HP to be destroyed after the three-unit attack." "Solution: the warrior and tank must attack by hand-to-hand combat, and the mage must use his skill." :!type "Text") _ui_tutorialref)
  (`UserWidget.AddToViewport` _ui_tutorialref 0))

(event `LeaderPassive`
  (bind _ui_tutorialref (`self.UI_TutorialRef`))
  ;[1 1 1] Set Tutorial Lines on widget
  (`self.InitUI`)
  (set `/Game/Core/Blueprints/Widget/Tutorial/WBP_Tutorial.TutorialLines` (`|MakeArray` "The commander is a special unit that costs more resources than basic units." "It has a passive skill that assists other units 2 squares away or less, depending on its affiliation (angel or demon)." "The angel commander heals nearby allied units at the start of each turn, and the demon commander increases the attack of nearby allied units as long as they are within a radius." "Use your warrior and demon commander to eliminate the enemy warrior." "Note: the enemy warrior has just enough HP to survive a normal attack by the player warrior." "Solution: move both units so that the warrior is close to the enemy and two squares from the commander, then attack." :!type "Text") _ui_tutorialref)
  (`UserWidget.AddToViewport` _ui_tutorialref 0))

(fn `InitUI`
  (bind _asbp_dc_custom_player_controller (cast `/Game/Core/Blueprints/BP_DC_CustomPlayerController` (`GameplayStatics.GetPlayerController` 0)))
  (bind _wbp_hud_ref (`/Game/Core/Blueprints/BP_DC_CustomPlayerController.WBP_HUD_Ref` _asbp_dc_custom_player_controller))
  (`/Game/Core/Blueprints/Widget/HUD/WBP_HUD.PushWidget` _wbp_hud_ref (`/Game/Core/Blueprints/Widget/HUD/WBP_HUD.WidgetStack_HUD` _wbp_hud_ref) "/Game/Core/Blueprints/Widget/Tutorial/WBP_Tutorial.WBP_Tutorial_C")
  (bind _aswbp_tutorial (cast `/Game/Core/Blueprints/Widget/Tutorial/WBP_Tutorial` (`/Game/Core/Blueprints/Widget/HUD/WBP_HUD.PushedWidget` _wbp_hud_ref)))
  (set `self.UI_TutorialRef` _aswbp_tutorial))

(fn `UserConstructionScript`)