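; Game instance that handles multiplayer sessions and runs the countdown for a turn-based match.
; Advanced Sessions creates, finds and joins two-slot LAN sessions filtered by a server name key, with the host opening the lobby as a listen server.
; A looping one-second timer drives the countdown, flipping each player controller's active turn when it expires, and pauses at game end to show the end screen.
; Event dispatchers announce found sessions, timer updates and turn changes.
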(event `CreateSession`
  (bind _returnvalue (`GameplayStatics.GetPlayerController` 0))
  ;[1 1 1] Advanced Session
  (`EndSessionCallbackProxy.EndSession` _returnvalue
    (:`then`
      (`DestroySessionCallbackProxy.DestroySession` _returnvalue
        (:`then`
          (`AdvancedSteamFriendsLibrary.GetSteamPersonaName` (`AdvancedSessionsLibrary.GetUniqueNetID` _returnvalue))
          (`CreateSessionCallbackProxyAdvanced.CreateAdvancedSession` (`|MakeArray` (`AdvancedSessionsLibrary.MakeLiteralSessionPropertyString` "ServerName" "CimeArtGame") (struct)) (`GameplayStatics.GetPlayerController` 0) 2 0 true
            (:`OnSuccess`
              (`GameplayStatics.OpenLevelBySoftObjectPtr` "/Game/Maps/LVL_Lobby.LVL_Lobby" true "listen"))))))))

(event `JoinSession`
  (params (`Actual Session` :type "BlueprintSessionResult Structure"))
  ;[1 1 1] Advanced Session
  (set `self.Actual Session` `Actual Session`)
  (`JoinSessionCallbackProxy.JoinSession` (`GameplayStatics.GetPlayerController` 0) (`self.Actual Session`)
    (:`OnSuccess`
      (`KismetSystemLibrary.PrintString` "Joined"))))

(event `FindSession`
  ;[1 1 1] Advanced Session
  (`KismetSystemLibrary.PrintString` "Launched")
  (bind _results (`FindSessionsCallbackProxyAdvanced.FindSessionsAdvanced` (`GameplayStatics.GetPlayerController` 0) 20000 true "AllServers" (`|MakeArray` (`AdvancedSessionsLibrary.MakeLiteralSessionSearchProperty` (`AdvancedSessionsLibrary.MakeLiteralSessionPropertyString` "ServerName" "CimeArtGame") "Equals")))
    (:`OnSuccess`
      (bind _output_get (set `self.SessionResults` _results))
      (`self.ED_SessionFound`)
      (`KismetSystemLibrary.PrintString` (`KismetStringLibrary.Conv_IntToString` (`KismetArrayLibrary.Array_Length` _output_get))))))

(event `SetTimer`
  ;[1 1 1] Timer
  (if (> (`self.Seconds`) 0)
    (`/Engine/EditorBlueprintResources/StandardMacros.DecrementInt` (`self.Seconds`)
      (:`  `
        (`self.ED_UpdateUI`)))
    (elif (> (`self.Minutes`) 0)
      (`/Engine/EditorBlueprintResources/StandardMacros.DecrementInt` (`self.Minutes`)
        (:`  `
          (set `self.Seconds` 59)
          (`self.ED_UpdateUI`)))
      (elif (not (and (== (`self.Minutes`) 0) (== (`self.Seconds`) 0)))
        (set `self.Minutes` 0)
        (set `self.Seconds` 59)
        (`self.ED_UpdateUI`)
        (else
          (`self.ChangeTurn`))))))

(event `StartGame`
  ;[1 1 1] Start Game
  (set `self.Minutes` 2)
  (set `self.Seconds` 0)
  (set `self.Turn` 1)
  (bind _returnvalue (`KismetSystemLibrary.K2_SetTimerDelegate` (`|CreateDelegate` :!event `SetTimer`) 1.0 true))
  (bind _output_get (set `self.TimerEvent` _returnvalue))
  (`KismetSystemLibrary.K2_UnPauseTimerHandle` _output_get))

(event `EndGame`
  ;[1 1 1] End Game
  (`KismetSystemLibrary.K2_PauseTimerHandle` (`self.TimerEvent`))
  (`WidgetLayoutLibrary.RemoveAllWidgets`)
  (bind _returnvalue (`|CreateWidget` "/Game/Blueprints/Widget/HUD/WBP_EndLevel.WBP_EndLevel_C"))
  (`UserWidget.AddToViewport` _returnvalue 0))

(event `ChangeTurn`
  ;[1 1 1] Change Turn
  (for _array_element (`GameStateBase.PlayerArray` (`GameplayStatics.GetGameState`))
    (bind _ascustom_player_controller (cast `CustomPlayerController` (`PlayerState.GetPlayerController` _array_element)))
    (bind _returnvalue (`CustomPlayerController.GetIsInActiveTurn` _ascustom_player_controller))
    (`CustomPlayerController.SetIsInActiveTurn` _ascustom_player_controller (select `bool` _returnvalue :`false` true)))
  (`/Engine/EditorBlueprintResources/StandardMacros.IncrementInt` (`self.Turn`)
    (:`  `
      (set `self.Minutes` 2)
      (set `self.Seconds` 0)
      (`self.ED_UpdateUI`)
      (`self.ED_UI_Turn`))))