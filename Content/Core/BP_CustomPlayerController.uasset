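; Custom player controller that handles UI navigation through Enhanced Input, adding a UI navigation mapping context on BeginPlay.
; Directional actions step wrapping vertical and horizontal indices sharing one max, while next/previous actions cycle a window index.
; Event dispatchers broadcast focus updates, window changes and back-to-close requests, leaving the response to listeners.
; Debug prints show the window index and its maximum every tick, plus a message on next window.
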(event `self.ReceiveBeginPlay`
  ;[1 1 1] Event Construct
  (`EnhancedInputSubsystemInterface.AddMappingContext` (pcsubsystem `EnhancedInputLocalPlayerSubsystem` (`GameplayStatics.GetPlayerController` 0)) "/Game/Core/Controller/IMC_UINavigation.IMC_UINavigation" 0 (struct)))

(event `EnhancedInput|/Game/Core/Controller/Inputs/UI_Navigation/IA_Up`
  (params (ActionValue :type Boolean) (ElapsedSeconds :type "Float (double-precision)") (TriggeredSeconds :type "Float (double-precision)") (InputAction :type "InputAction Object Reference" :default "/Game/Core/Controller/Inputs/UI_Navigation/IA_Up.IA_Up"))
  ;[1 1 1] UI Navigation : Up and Down
  (:`Triggered`
    (if (> (`self.VerticalIndex`) 0)
      (`/Engine/EditorBlueprintResources/StandardMacros.DecrementInt` (`self.VerticalIndex`)
        (:`  `
          _))
      (else
        (set `self.VerticalIndex` (`self.MaxIndex`))))
    (`self.ED_UpdateFocus`)))

(event `EnhancedInput|/Game/Core/Controller/Inputs/UI_Navigation/IA_Left`
  (params (ActionValue :type Boolean) (ElapsedSeconds :type "Float (double-precision)") (TriggeredSeconds :type "Float (double-precision)") (InputAction :type "InputAction Object Reference" :default "/Game/Core/Controller/Inputs/UI_Navigation/IA_Left.IA_Left"))
  ;[1 1 1] UI Navigation : Left and Right
  (:`Triggered`
    (if (> (`self.HorizontalIndex`) 0)
      (`/Engine/EditorBlueprintResources/StandardMacros.DecrementInt` (`self.HorizontalIndex`)
        (:`  `
          _))
      (else
        (set `self.HorizontalIndex` (`self.MaxIndex`))))
    (`self.ED_UpdateFocus`)))

(event `EnhancedInput|/Game/Core/Controller/Inputs/UI_Navigation/IA_Down`
  (params (ActionValue :type Boolean) (ElapsedSeconds :type "Float (double-precision)") (TriggeredSeconds :type "Float (double-precision)") (InputAction :type "InputAction Object Reference" :default "/Game/Core/Controller/Inputs/UI_Navigation/IA_Down.IA_Down"))
  ;[1 1 1] UI Navigation : Up and Down
  (:`Triggered`
    (if (< (`self.VerticalIndex`) (`self.MaxIndex`))
      (`/Engine/EditorBlueprintResources/StandardMacros.IncrementInt` (`self.VerticalIndex`)
        (:`  `
          _))
      (else
        (set `self.VerticalIndex` 0)))
    (`self.ED_UpdateFocus`)))

(event `EnhancedInput|/Game/Core/Controller/Inputs/UI_Navigation/IA_Right`
  (params (ActionValue :type Boolean) (ElapsedSeconds :type "Float (double-precision)") (TriggeredSeconds :type "Float (double-precision)") (InputAction :type "InputAction Object Reference" :default "/Game/Core/Controller/Inputs/UI_Navigation/IA_Right.IA_Right"))
  ;[1 1 1] UI Navigation : Left and Right
  (:`Triggered`
    (if (< (`self.HorizontalIndex`) (`self.MaxIndex`))
      (`/Engine/EditorBlueprintResources/StandardMacros.IncrementInt` (`self.HorizontalIndex`)
        (:`  `
          _))
      (else
        (set `self.HorizontalIndex` 0)))
    (`self.ED_UpdateFocus`)))

(event `EnhancedInput|/Game/Core/Controller/Inputs/UI_Navigation/IA_NextWindow`
  (params (ActionValue :type Boolean) (ElapsedSeconds :type "Float (double-precision)") (TriggeredSeconds :type "Float (double-precision)") (InputAction :type "InputAction Object Reference" :default "/Game/Core/Controller/Inputs/UI_Navigation/IA_NextWindow.IA_NextWindow"))
  ;[1 1 1] UI Navigation : Change Window
  (:`Triggered`
    (`KismetSystemLibrary.PrintString` "Hello")
    (if (< (`self.WindowIndex`) (`self.MaxWindowIndex`))
      (`/Engine/EditorBlueprintResources/StandardMacros.IncrementInt` (`self.WindowIndex`)
        (:`  `
          _))
      (else
        (set `self.WindowIndex` 0)))
    (`self.ED_ChangeWindow`)))

(event `EnhancedInput|/Game/Core/Controller/Inputs/UI_Navigation/IA_PreviousWindow`
  (params (ActionValue :type Boolean) (ElapsedSeconds :type "Float (double-precision)") (TriggeredSeconds :type "Float (double-precision)") (InputAction :type "InputAction Object Reference" :default "/Game/Core/Controller/Inputs/UI_Navigation/IA_PreviousWindow.IA_PreviousWindow"))
  ;[1 1 1] UI Navigation : Change Window
  (:`Triggered`
    (if (> (`self.WindowIndex`) 0)
      (`/Engine/EditorBlueprintResources/StandardMacros.DecrementInt` (`self.WindowIndex`)
        (:`  `
          _))
      (else
        (set `self.WindowIndex` (`self.MaxWindowIndex`))))
    (`self.ED_ChangeWindow`)))

(event `EnhancedInput|/Game/Core/Controller/Inputs/UI_Navigation/IA_Back`
  (params (ActionValue :type Boolean) (ElapsedSeconds :type "Float (double-precision)") (TriggeredSeconds :type "Float (double-precision)") (InputAction :type "InputAction Object Reference" :default "/Game/Core/Controller/Inputs/UI_Navigation/IA_Back.IA_Back"))
  ;[1 1 1] UI Navigation : Back
  (:`Triggered`
    (`self.ED_CloseWidget`)))

(event `self.ReceiveTick`
  (params (DeltaSeconds :type "Float (single-precision)"))
  (`KismetSystemLibrary.PrintString` (`KismetStringLibrary.Concat_StrStr` "Current : " (`KismetStringLibrary.Conv_IntToString` (`self.WindowIndex`))))
  (`KismetSystemLibrary.PrintString` (`KismetStringLibrary.Concat_StrStr` "Max : " (`KismetStringLibrary.Conv_IntToString` (`self.MaxWindowIndex`)))))

(fn `UserConstructionScript`)