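; Lobby game mode that handles player logins and decides where each joining player spawns.
; On PostLogin it casts the new controller to PC_Lobby and calls its OCHandleLogin, passing the controller itself.
; The ChoosePlayerStart override gives each player the PlayerStart whose tag equals their index in the GameState's PlayerArray.
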(event `self.K2_PostLogin`
  (params (NewPlayer :type "PlayerController Object Reference"))
  (bind _aspc_lobby (cast `/Game/Blueprints/Lobby/PC_Lobby` NewPlayer))
  (`/Game/Blueprints/Lobby/PC_Lobby.OC_HandleLogin` _aspc_lobby _aspc_lobby))

(fn `ChoosePlayerStart`
  (params (Player :type "Controller Object Reference"))
  (returns (ReturnValue :type "Actor Object Reference"))
  (bind _outactors (`GameplayStatics.GetAllActorsOfClass` "/Script/Engine.PlayerStart"))
  (for _array_element _outactors
    (if (== (`PlayerStart.PlayerStartTag` _array_element) (`KismetStringLibrary.Conv_StringToName` (`KismetStringLibrary.Conv_IntToString` (`KismetArrayLibrary.Array_Find` (`GameStateBase.PlayerArray` (`GameplayStatics.GetGameState`)) (`Controller.PlayerState` Player)))))
      (return _array_element))))

(fn `UserConstructionScript`)