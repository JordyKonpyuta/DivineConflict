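; Lobby player Blueprint that keeps its Widget component's rotation aligned to the camera's line of sight.
; Every Tick, UpdateWidgetRotation looks up a CameraActor with GetActorOfClass and, if valid, sets the widget's world rotation to the look-at rotation from the camera to the widget.
; The widget's forward axis therefore points away from the camera, and the actor lookup repeats each frame.
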(event `self.ReceiveTick`
  (params (DeltaSeconds :type "Float (single-precision)"))
  (`self.UpdateWidgetRotation`))

(fn `UpdateWidgetRotation`
  (bind _returnvalue (`GameplayStatics.GetActorOfClass` "/Script/Engine.CameraActor"))
  (`/Engine/EditorBlueprintResources/StandardMacros.IsValid` _returnvalue
    (:`Is Valid`
      (bind (_returnvalue_roll _returnvalue_pitch _returnvalue_yaw) (`KismetMathLibrary.BreakRotator` (`KismetMathLibrary.FindLookAtRotation` (`self.K2_GetActorLocation` _returnvalue) (`SceneComponent.K2_GetComponentLocation` (`self.Widget`)))))
      (`SceneComponent.K2_SetWorldRotation` (`self.Widget`) (`KismetMathLibrary.MakeRotator` _returnvalue_roll _returnvalue_pitch _returnvalue_yaw) false false))))

(fn `UserConstructionScript`)